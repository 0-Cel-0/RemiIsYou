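; Baball is a short-lived actor spawned around the player Baba that drifts and scales before vanishing, apparently a movement puff effect.
; On BeginPlay it reads Baba's LastMove once and plays the BaballShrink timeline.
; Each update scales the actor between zero and full size by the track value and nudges it along X or Y according to that move direction.
; When the timeline finishes, the actor destroys itself.
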(event `self.ReceiveBeginPlay`
  (bind (_returnvalue_x _returnvalue_y _returnvalue_z) (`KismetMathLibrary.BreakVector` (`self.K2_GetActorLocation`)))
  (`/Engine/EditorBlueprintResources/StandardMacros.DoOnce` false
    (:`Completed`
      (bind _asbaba (cast `/Game/Blueprint/Baba` (`GameplayStatics.GetPlayerCharacter` 0)))
      (set `self.LocalLastMove` (`/Game/Blueprint/Baba.LastMove` _asbaba))
      (bind (_direction _newtrack_0) (`Timeline|BaballShrink` :!via `PlayFromStart`)
        (:`Update`
          (`self.SetActorScale3D` (`KismetMathLibrary.VLerp` (0.0 0.0 0.0) (1.0 1.0 1.0) _newtrack_0))
          (switch `int` (`self.LocalLastMove`)
            (:`0`
              (bind _returnvalue (* _newtrack_0 2.0))
              (`self.K2_SetActorLocation` (`KismetMathLibrary.MakeVector` _returnvalue_x (+ _returnvalue _returnvalue_y) _returnvalue_z)))
            (:`1`
              (bind _returnvalue_2 (* _newtrack_0 -2.0))
              (`self.K2_SetActorLocation` (`KismetMathLibrary.MakeVector` _returnvalue_x (+ _returnvalue_2 _returnvalue_y) _returnvalue_z)))
            (:`2`
              (`self.K2_SetActorLocation` (`KismetMathLibrary.MakeVector` (+ _returnvalue _returnvalue_x) _returnvalue_y _returnvalue_z)))
            (:`3`
              (`self.K2_SetActorLocation` (`KismetMathLibrary.MakeVector` (+ _returnvalue_2 _returnvalue_x) _returnvalue_y _returnvalue_z)))))
        (:`Finished`
          (`self.K2_DestroyActor`))))))

(fn `UserConstructionScript`)