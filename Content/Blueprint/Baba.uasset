(event `self.UpCheck.OnComponentBeginOverlap`
  (params (OverlappedComponent :type "PrimitiveComponent Object Reference") (OtherActor :type "Actor Object Reference") (OtherComp :type "PrimitiveComponent Object Reference") (OtherBodyIndex :type Integer) (bFromSweep :type Boolean) (SweepResult :type "HitResult Structure (by ref)"))
  ;[1 0.483 0.477] Check & Store Adjacent Blocks
  (cast `/Game/Blueprint/TextBaba` OtherActor
    (:`then`
      (set `self.CanGoUp` false))
    (:`CastFailed`
      (bind _asrock (cast `/Game/Blueprint/Rock` OtherActor))
      (set `self.As Up Rock` _asrock)
      (set `self.RockOnTheTop` true))))

(event `self.UpCheck.OnComponentEndOverlap`
  (params (OverlappedComponent :type "PrimitiveComponent Object Reference") (OtherActor :type "Actor Object Reference") (OtherComp :type "PrimitiveComponent Object Reference") (OtherBodyIndex :type Integer))
  ;[1 0.483 0.477] Check & Store Adjacent Blocks
  (cast `/Game/Blueprint/TextBaba` OtherActor
    (:`then`
      (set `self.CanGoUp` true))
    (:`CastFailed`
      (cast `/Game/Blueprint/Rock` OtherActor)
      (set `self.RockOnTheTop` false))))

(event `self.DownCheck.OnComponentBeginOverlap`
  (params (OverlappedComponent :type "PrimitiveComponent Object Reference") (OtherActor :type "Actor Object Reference") (OtherComp :type "PrimitiveComponent Object Reference") (OtherBodyIndex :type Integer) (bFromSweep :type Boolean) (SweepResult :type "HitResult Structure (by ref)"))
  ;[1 0.483 0.477] Check & Store Adjacent Blocks
  (cast `/Game/Blueprint/TextBaba` OtherActor
    (:`then`
      (set `self.CanGoDown` false))
    (:`CastFailed`
      (bind _asrock (cast `/Game/Blueprint/Rock` OtherActor))
      (set `self.As Down Rock` _asrock)
      (set `self.RockOnTheBottom` true))))

(event `self.DownCheck.OnComponentEndOverlap`
  (params (OverlappedComponent :type "PrimitiveComponent Object Reference") (OtherActor :type "Actor Object Reference") (OtherComp :type "PrimitiveComponent Object Reference") (OtherBodyIndex :type Integer))
  ;[1 0.483 0.477] Check & Store Adjacent Blocks
  (cast `/Game/Blueprint/TextBaba` OtherActor
    (:`then`
      (set `self.CanGoDown` true))
    (:`CastFailed`
      (cast `/Game/Blueprint/Rock` OtherActor)
      (set `self.RockOnTheBottom` false))))

(event `self.LeftCheck.OnComponentBeginOverlap`
  (params (OverlappedComponent :type "PrimitiveComponent Object Reference") (OtherActor :type "Actor Object Reference") (OtherComp :type "PrimitiveComponent Object Reference") (OtherBodyIndex :type Integer) (bFromSweep :type Boolean) (SweepResult :type "HitResult Structure (by ref)"))
  ;[1 0.483 0.477] Check & Store Adjacent Blocks
  (cast `/Game/Blueprint/TextBaba` OtherActor
    (:`then`
      (set `self.CanGoLeft` false))
    (:`CastFailed`
      (bind _asrock (cast `/Game/Blueprint/Rock` OtherActor))
      (set `self.As Left Rock` _asrock)
      (set `self.RockOnTheLeft` true))))

(event `Key|R`
  (params (Key :type "Key Structure"))
  ;[1 0 0] ResetLevel
  (:`Pressed`
    (`/Engine/EditorBlueprintResources/StandardMacros.DoOnce` false
      (:`Completed`
        (`GameplayStatics.PlaySound2D` "/Game/Assets/Audio/SC_RestartSoundBaba.SC_RestartSoundBaba" 1.0 1.0 0.0 null null)
        (`KismetSystemLibrary.K2_SetTimerDelegate` (`|CreateDelegate` :!event `RestartLevel`) 2.0)
        (bind _returnvalue (`|CreateWidget` "/Game/UI/WBP_Curtain.WBP_Curtain_C"))
        (bind _output_get (set `self.Curtain` _returnvalue))
        (`UserWidget.AddToViewport` _output_get 0)
        (`/Game/UI/WBP_Curtain.PlayCurtain` (`self.Curtain`))))))

(event `self.LeftCheck.OnComponentEndOverlap`
  (params (OverlappedComponent :type "PrimitiveComponent Object Reference") (OtherActor :type "Actor Object Reference") (OtherComp :type "PrimitiveComponent Object Reference") (OtherBodyIndex :type Integer))
  ;[1 0.483 0.477] Check & Store Adjacent Blocks
  (cast `/Game/Blueprint/TextBaba` OtherActor
    (:`then`
      (set `self.CanGoLeft` true))
    (:`CastFailed`
      (cast `/Game/Blueprint/Rock` OtherActor)
      (set `self.RockOnTheLeft` false))))

(event `RestartLevel`
  ;[1 0 0] ResetLevel
  (`GameplayStatics.OpenLevelBySoftObjectPtr` "/Game/Maps/RemiIsYouLevel00.RemiIsYouLevel00"))

(event `self.RightCheck.OnComponentBeginOverlap`
  (params (OverlappedComponent :type "PrimitiveComponent Object Reference") (OtherActor :type "Actor Object Reference") (OtherComp :type "PrimitiveComponent Object Reference") (OtherBodyIndex :type Integer) (bFromSweep :type Boolean) (SweepResult :type "HitResult Structure (by ref)"))
  ;[1 0.483 0.477] Check & Store Adjacent Blocks
  (cast `/Game/Blueprint/TextBaba` OtherActor
    (:`then`
      (set `self.CanGoRight` false))
    (:`CastFailed`
      (bind _asrock (cast `/Game/Blueprint/Rock` OtherActor))
      (set `self.As Right Rock` _asrock)
      (set `self.RockOnTheRight` true))))

(event `PlayStepSound`
  ;[0.5 0 1] PlayStepSound
  (`GameplayStatics.PlaySound2D` "/Game/Assets/Audio/SC_StepSoundBaba.SC_StepSoundBaba" 1.0 1.0 0.0 null null))

(event `self.ReceiveBeginPlay`
  ;[0 0 0] Begin Play
  (bind _asplayer_controller (cast `PlayerController` (`self.GetController`)))
  (message `EnhancedInputSubsystemInterface.AddMappingContext` (pcsubsystem `EnhancedInputLocalPlayerSubsystem` _asplayer_controller) "/Game/Blueprint/Inputs/IMC_Baba.IMC_Baba" 0 (struct)))

(event `Increase Movement Cycle`
  (bind _movementcycle (`self.MovementCycle`))
  ;[0 1 0.5] Increase Movement Cycle
  (switch `int` _movementcycle
    (:`Default`
      (`/Engine/EditorBlueprintResources/StandardMacros.IncrementInt` _movementcycle :!label _label))
    (:`0`
      (goto _label))
    (:`1`
      (goto _label))
    (:`2`
      (goto _label))
    (:`3`
      (set `self.MovementCycle` 0))))

(event `self.RightCheck.OnComponentEndOverlap`
  (params (OverlappedComponent :type "PrimitiveComponent Object Reference") (OtherActor :type "Actor Object Reference") (OtherComp :type "PrimitiveComponent Object Reference") (OtherBodyIndex :type Integer))
  ;[1 0.483 0.477] Check & Store Adjacent Blocks
  (cast `/Game/Blueprint/TextBaba` OtherActor
    (:`then`
      (set `self.CanGoRight` true))
    (:`CastFailed`
      (cast `/Game/Blueprint/Rock` OtherActor)
      (set `self.RockOnTheRight` false))))

(event `is Win`
  ;[1 0.9096 0] Win
  (set `self.UnableToMove` true))

(event `EnhancedInput|/Game/Blueprint/Inputs/IA_UpBaba`
  (params (ActionValue :type Boolean) (ElapsedSeconds :type "Float (double-precision)") (TriggeredSeconds :type "Float (double-precision)") (InputAction :type "InputAction Object Reference" :default "/Game/Blueprint/Inputs/IA_UpBaba.IA_UpBaba"))
  (bind _timerup (`self.TimerUp`))
  ;[0.5 0.5 0.5] InputUp
  (:`Started`
    (bind _returnvalue (`KismetSystemLibrary.K2_SetTimerDelegate` (`|CreateDelegate` :!event `up`) 0.15 true -0.15))
    (set `self.TimerUp` _returnvalue))
  (:`Completed`
    (`KismetSystemLibrary.K2_PauseTimerHandle` _timerup)
    (`KismetSystemLibrary.K2_ClearAndInvalidateTimerHandle` _timerup)))

(event `Up`
  (bind _capsulecomponent (`self.CapsuleComponent`))
  (bind (_returnvalue_x _returnvalue_y _returnvalue_z) (`KismetMathLibrary.BreakVector` (`SceneComponent.K2_GetComponentLocation` (`self.CapsuleComponent`))))
  (bind (_returnvalue_x_2 _returnvalue_y_2 _returnvalue_z_2) (`KismetMathLibrary.BreakVector` (`SceneComponent.K2_GetComponentLocation` _capsulecomponent)))
  ;[0.2 0.2 0.2] Up
  (if (not (`self.UnableToMove`))
    (`self.Set Flipbook Up`)
    (if (`self.CanGoUp`)
      (if (<= _returnvalue_y_2 -750.0)
        (`SceneComponent.K2_SetWorldLocation` _capsulecomponent (`KismetMathLibrary.MakeVector` _returnvalue_x_2 -750.0 _returnvalue_z_2) false false)
        (elif (`self.RockOnTheTop`)
          (`self.MoveRockUp`)
          (else
            (set `self.LastMove` 0 :!label _label_2)
            (`|SpawnActorFromClass` "/Game/Blueprint/Baball.Baball_C" (`KismetMathLibrary.MakeTransform` (`KismetMathLibrary.MakeVector` _returnvalue_x_2 _returnvalue_y_2)) "Undefined" "MultiplyWithRoot" null null)
            (`self.PlayStepSound`)
            (`SceneComponent.K2_SetWorldLocation` (`self.CapsuleComponent`) (`KismetMathLibrary.MakeVector` _returnvalue_x (+ _returnvalue_y -100.0) _returnvalue_z) false false)
            (`self.Increase Movement Cycle`)))))))

(event `MoveRockUp`
  (bind _as_up_rock (`self.As Up Rock`))
  (bind _as_up_rock_2 (`self.As Up Rock`))
  (bind _blockid (`/Game/Blueprint/Rock.BlockID` _as_up_rock_2))
  (bind (_returnvalue_x _returnvalue_y _returnvalue_z) (`KismetMathLibrary.BreakVector` (`SceneComponent.K2_GetComponentLocation` (`Actor.RootComponent` (`self.As Up Rock`)))))
  ;[1 0.483 0.477] MoveRockUp
  (if (or (== _blockid 5) (== _blockid 6))
    _
    (elif (not (`/Game/Blueprint/Rock.Pushable` _as_up_rock_2))
      (`/Game/Blueprint/Rock.CheckNextToWall` _as_up_rock :!label _label_3)
      (`/Game/Blueprint/Rock.Is Sentence Valid` _as_up_rock)
      (`self.RockMovedUp`)
      (`/Game/Blueprint/Rock.Check if Sentence` _as_up_rock)
      (elif (not (<= _returnvalue_y -750.0))
        (`self.K2_SetActorLocation` (`self.As Up Rock`) (`KismetMathLibrary.MakeVector` _returnvalue_x (+ _returnvalue_y -100.0) _returnvalue_z) false false)
        (goto _label_3)))))

(event `Set Flipbook Right`
  (bind _babadisplay (`self.BabaDisplay`))
  ;[0 1 0.5] Set Flipbook
  (switch `int` (`self.MovementCycle`)
    (:`Default`
      (`PaperFlipbookComponent.SetFlipbook` _babadisplay "/Game/Sprites/Baba/BabaRight01.BabaRight01" :!label _label_4))
    (:`0`
      (goto _label_4))
    (:`1`
      (`PaperFlipbookComponent.SetFlipbook` _babadisplay "/Game/Sprites/Baba/BabaRight02.BabaRight02"))
    (:`2`
      (`PaperFlipbookComponent.SetFlipbook` _babadisplay "/Game/Sprites/Baba/BabaRight03.BabaRight03"))
    (:`3`
      (`PaperFlipbookComponent.SetFlipbook` _babadisplay "/Game/Sprites/Baba/BabaRight04.BabaRight04"))))

(event `Set Flipbook Up`
  (bind _babadisplay (`self.BabaDisplay`))
  ;[0 1 0.5] Set Flipbook
  (switch `int` (`self.MovementCycle`)
    (:`Default`
      (`PaperFlipbookComponent.SetFlipbook` _babadisplay "/Game/Sprites/Baba/BabaUp01.BabaUp01" :!label _label_5))
    (:`0`
      (goto _label_5))
    (:`1`
      (`PaperFlipbookComponent.SetFlipbook` _babadisplay "/Game/Sprites/Baba/BabaUp02.BabaUp02"))
    (:`2`
      (`PaperFlipbookComponent.SetFlipbook` _babadisplay "/Game/Sprites/Baba/BabaUp03.BabaUp03"))
    (:`3`
      (`PaperFlipbookComponent.SetFlipbook` _babadisplay "/Game/Sprites/Baba/BabaUp04.BabaUp04"))))

(event `RockMovedUp`
  ;[0.2 0.2 0.2] Up
  (goto _label_2))

(event `EnhancedInput|/Game/Blueprint/Inputs/IA_DownBaba`
  (params (ActionValue :type Boolean) (ElapsedSeconds :type "Float (double-precision)") (TriggeredSeconds :type "Float (double-precision)") (InputAction :type "InputAction Object Reference" :default "/Game/Blueprint/Inputs/IA_DownBaba.IA_DownBaba"))
  (bind _timerdown (`self.TimerDown`))
  ;[0.5 0.5 0.5] InputDown
  (:`Started`
    (bind _returnvalue (`KismetSystemLibrary.K2_SetTimerDelegate` (`|CreateDelegate` :!event `Down`) 0.15 true -0.15))
    (set `self.TimerDown` _returnvalue))
  (:`Completed`
    (`KismetSystemLibrary.K2_PauseTimerHandle` _timerdown)
    (`KismetSystemLibrary.K2_ClearAndInvalidateTimerHandle` _timerdown)))

(event `Down`
  (bind _capsulecomponent (`self.CapsuleComponent`))
  (bind (_returnvalue_x _returnvalue_y _returnvalue_z) (`KismetMathLibrary.BreakVector` (`SceneComponent.K2_GetComponentLocation` (`self.CapsuleComponent`))))
  (bind (_returnvalue_x_2 _returnvalue_y_2 _returnvalue_z_2) (`KismetMathLibrary.BreakVector` (`SceneComponent.K2_GetComponentLocation` _capsulecomponent)))
  ;[0.2 0.2 0.2] Down
  (if (not (`self.UnableToMove`))
    (`self.Set Flipbook Down`)
    (if (`self.CanGoDown`)
      (if (>= _returnvalue_y_2 750.0)
        (`SceneComponent.K2_SetWorldLocation` _capsulecomponent (`KismetMathLibrary.MakeVector` _returnvalue_x_2 750.0 _returnvalue_z_2) false false)
        (elif (`self.RockOnTheBottom`)
          (`self.MoveRockDown`)
          (else
            (set `self.LastMove` 1 :!label _label_6)
            (`|SpawnActorFromClass` "/Game/Blueprint/Baball.Baball_C" (`KismetMathLibrary.MakeTransform` (`KismetMathLibrary.MakeVector` _returnvalue_x_2 _returnvalue_y_2)) "Undefined" "MultiplyWithRoot" null null)
            (`self.PlayStepSound`)
            (`SceneComponent.K2_SetWorldLocation` (`self.CapsuleComponent`) (`KismetMathLibrary.MakeVector` _returnvalue_x (+ _returnvalue_y 100.0) _returnvalue_z) false false)
            (`self.Increase Movement Cycle`)))))))

(event `MoveRockDown`
  (bind _as_down_rock (`self.As Down Rock`))
  (bind (_returnvalue_x _returnvalue_y _returnvalue_z) (`KismetMathLibrary.BreakVector` (`SceneComponent.K2_GetComponentLocation` (`Actor.RootComponent` (`self.As Down Rock`)))))
  ;[1 0.483 0.477] MoveRockDown
  (if (not (`/Game/Blueprint/Rock.Pushable` (`self.As Down Rock`)))
    (`/Game/Blueprint/Rock.CheckNextToWall` _as_down_rock :!label _label_7)
    (`/Game/Blueprint/Rock.Is Sentence Valid` _as_down_rock)
    (`self.RockMovedDown`)
    (`/Game/Blueprint/Rock.Check if Sentence` _as_down_rock)
    (elif (not (>= _returnvalue_y 750.0))
      (`self.K2_SetActorLocation` (`self.As Down Rock`) (`KismetMathLibrary.MakeVector` _returnvalue_x (+ _returnvalue_y 100.0) _returnvalue_z) false false)
      (goto _label_7))))

(event `Set Flipbook Left`
  (bind _babadisplay (`self.BabaDisplay`))
  ;[0 1 0.5] Set Flipbook
  (switch `int` (`self.MovementCycle`)
    (:`Default`
      (`PaperFlipbookComponent.SetFlipbook` _babadisplay "/Game/Sprites/Baba/BabaLeft01.BabaLeft01" :!label _label_8))
    (:`0`
      (goto _label_8))
    (:`1`
      (`PaperFlipbookComponent.SetFlipbook` _babadisplay "/Game/Sprites/Baba/BabaLeft02.BabaLeft02"))
    (:`2`
      (`PaperFlipbookComponent.SetFlipbook` _babadisplay "/Game/Sprites/Baba/BabaLeft03.BabaLeft03"))
    (:`3`
      (`PaperFlipbookComponent.SetFlipbook` _babadisplay "/Game/Sprites/Baba/BabaLeft04.BabaLeft04"))))

(event `Set Flipbook Down`
  (bind _babadisplay (`self.BabaDisplay`))
  ;[0 1 0.5] Set Flipbook
  (switch `int` (`self.MovementCycle`)
    (:`Default`
      (`PaperFlipbookComponent.SetFlipbook` _babadisplay "/Game/Sprites/Baba/BabaDown01.BabaDown01" :!label _label_9))
    (:`0`
      (goto _label_9))
    (:`1`
      (`PaperFlipbookComponent.SetFlipbook` _babadisplay "/Game/Sprites/Baba/BabaDown02.BabaDown02"))
    (:`2`
      (`PaperFlipbookComponent.SetFlipbook` _babadisplay "/Game/Sprites/Baba/BabaDown03.BabaDown03"))
    (:`3`
      (`PaperFlipbookComponent.SetFlipbook` _babadisplay "/Game/Sprites/Baba/BabaDown04.BabaDown04"))))

(event `RockMovedDown`
  ;[0.2 0.2 0.2] Down
  (goto _label_6))

(event `EnhancedInput|/Game/Blueprint/Inputs/IA_LeftBaba`
  (params (ActionValue :type Boolean) (ElapsedSeconds :type "Float (double-precision)") (TriggeredSeconds :type "Float (double-precision)") (InputAction :type "InputAction Object Reference" :default "/Game/Blueprint/Inputs/IA_LeftBaba.IA_LeftBaba"))
  (bind _timerleft (`self.TimerLeft`))
  ;[0.5 0.5 0.5] InputLeft
  (:`Started`
    (bind _returnvalue (`KismetSystemLibrary.K2_SetTimerDelegate` (`|CreateDelegate` :!event `Left`) 0.15 true -0.15))
    (set `self.TimerLeft` _returnvalue))
  (:`Completed`
    (`KismetSystemLibrary.K2_PauseTimerHandle` _timerleft)
    (`KismetSystemLibrary.K2_ClearAndInvalidateTimerHandle` _timerleft)))

(event `Left`
  (bind _capsulecomponent (`self.CapsuleComponent`))
  (bind (_returnvalue_x _returnvalue_y _returnvalue_z) (`KismetMathLibrary.BreakVector` (`SceneComponent.K2_GetComponentLocation` (`self.CapsuleComponent`))))
  (bind (_returnvalue_x_2 _returnvalue_y_2 _returnvalue_z_2) (`KismetMathLibrary.BreakVector` (`SceneComponent.K2_GetComponentLocation` _capsulecomponent)))
  ;[0.2 0.2 0.2] Left
  (if (not (`self.UnableToMove`))
    (`self.Set Flipbook Left`)
    (if (`self.CanGoLeft`)
      (if (<= _returnvalue_x_2 -1550.0)
        (`SceneComponent.K2_SetWorldLocation` _capsulecomponent (`KismetMathLibrary.MakeVector` -1550.0 _returnvalue_y_2 _returnvalue_z_2) false false)
        (elif (`self.RockOnTheLeft`)
          (`self.MoveRockLeft`)
          (else
            (set `self.LastMove` 2 :!label _label_10)
            (`|SpawnActorFromClass` "/Game/Blueprint/Baball.Baball_C" (`KismetMathLibrary.MakeTransform` (`KismetMathLibrary.MakeVector` _returnvalue_x_2 (+ _returnvalue_y_2 20.0))) "Undefined" "MultiplyWithRoot" null null)
            (`self.PlayStepSound`)
            (`SceneComponent.K2_SetWorldLocation` (`self.CapsuleComponent`) (`KismetMathLibrary.MakeVector` (+ _returnvalue_x -100.0) _returnvalue_y _returnvalue_z) false false)
            (`self.Increase Movement Cycle`)))))))

(event `MoveRockLeft`
  (bind _as_left_rock (`self.As Left Rock`))
  (bind _as_left_rock_2 (`self.As Left Rock`))
  (bind (_returnvalue_x _returnvalue_y) (`KismetMathLibrary.BreakVector` (`self.K2_GetActorLocation` _as_left_rock_2)))
  (bind _blockid (`/Game/Blueprint/Rock.BlockID` _as_left_rock_2))
  (bind (_returnvalue_x_2 _returnvalue_y_2 _returnvalue_z) (`KismetMathLibrary.BreakVector` (`SceneComponent.K2_GetComponentLocation` (`Actor.RootComponent` (`self.As Left Rock`)))))
  ;[1 0.483 0.477] MoveRockLeft
  (if (or (== _blockid 2) (== _blockid 6) (and (== _blockid 1) (== _returnvalue_x -1450.0) (== _returnvalue_y -650.0)))
    _
    (elif (not (`/Game/Blueprint/Rock.Pushable` _as_left_rock_2))
      (`/Game/Blueprint/Rock.CheckNextToWall` _as_left_rock :!label _label_11)
      (`/Game/Blueprint/Rock.Is Sentence Valid` _as_left_rock)
      (`self.RockMovedLeft`)
      (`/Game/Blueprint/Rock.Check if Sentence` _as_left_rock)
      (elif (not (<= _returnvalue_x_2 -1550.0))
        (`self.K2_SetActorLocation` (`self.As Left Rock`) (`KismetMathLibrary.MakeVector` (+ _returnvalue_x_2 -100.0) _returnvalue_y_2 _returnvalue_z) false false)
        (goto _label_11)))))

(event `RockMovedLeft`
  ;[0.2 0.2 0.2] Left
  (goto _label_10))

(event `EnhancedInput|/Game/Blueprint/Inputs/IA_RightBaba`
  (params (ActionValue :type Boolean) (ElapsedSeconds :type "Float (double-precision)") (TriggeredSeconds :type "Float (double-precision)") (InputAction :type "InputAction Object Reference" :default "/Game/Blueprint/Inputs/IA_RightBaba.IA_RightBaba"))
  (bind _timerright (`self.TimerRight`))
  ;[0.5 0.5 0.5] InputRight
  (:`Started`
    (bind _returnvalue (`KismetSystemLibrary.K2_SetTimerDelegate` (`|CreateDelegate` :!event `Right`) 0.15 true -0.15))
    (set `self.TimerRight` _returnvalue))
  (:`Completed`
    (`KismetSystemLibrary.K2_PauseTimerHandle` _timerright)
    (`KismetSystemLibrary.K2_ClearAndInvalidateTimerHandle` _timerright)))

(event `Right`
  (bind _capsulecomponent (`self.CapsuleComponent`))
  (bind (_returnvalue_x _returnvalue_y _returnvalue_z) (`KismetMathLibrary.BreakVector` (`SceneComponent.K2_GetComponentLocation` _capsulecomponent)))
  (bind (_returnvalue_x_2 _returnvalue_y_2 _returnvalue_z_2) (`KismetMathLibrary.BreakVector` (`SceneComponent.K2_GetComponentLocation` (`self.CapsuleComponent`))))
  ;[0.2 0.2 0.2] Right
  (if (not (`self.UnableToMove`))
    (`self.Set Flipbook Right`)
    (if (`self.CanGoRight`)
      (if (>= _returnvalue_x 1550.0)
        (`SceneComponent.K2_SetWorldLocation` _capsulecomponent (`KismetMathLibrary.MakeVector` 1550.0 _returnvalue_y _returnvalue_z) false false)
        (elif (`self.RockOnTheRight`)
          (`self.MoveRockRight`)
          (else
            (set `self.LastMove` 3 :!label _label_12)
            (`|SpawnActorFromClass` "/Game/Blueprint/Baball.Baball_C" (`KismetMathLibrary.MakeTransform` (`KismetMathLibrary.MakeVector` _returnvalue_x (+ _returnvalue_y 20.0))) "Undefined" "MultiplyWithRoot" null null)
            (`self.PlayStepSound`)
            (`SceneComponent.K2_SetWorldLocation` (`self.CapsuleComponent`) (`KismetMathLibrary.MakeVector` (+ _returnvalue_x_2 100.0) _returnvalue_y_2 _returnvalue_z_2) false false)
            (`self.Increase Movement Cycle`)))))))

(event `MoveRockRight`
  (bind _as_right_rock (`self.As Right Rock`))
  (bind _as_right_rock_2 (`self.As Right Rock`))
  (bind (_returnvalue_x _returnvalue_y _returnvalue_z) (`KismetMathLibrary.BreakVector` (`SceneComponent.K2_GetComponentLocation` (`Actor.RootComponent` _as_right_rock_2))))
  ;[1 0.483 0.477] MoveRockRight
  (if (not (`/Game/Blueprint/Rock.Pushable` (`self.As Right Rock`)))
    (`/Game/Blueprint/Rock.CheckNextToWall` _as_right_rock :!label _label_13)
    (`/Game/Blueprint/Rock.Is Sentence Valid` _as_right_rock)
    (`self.RockMovedRight`)
    (`/Game/Blueprint/Rock.Check if Sentence` _as_right_rock)
    (elif (not (>= _returnvalue_x 1550.0))
      (`self.K2_SetActorLocation` _as_right_rock_2 (`KismetMathLibrary.MakeVector` (+ _returnvalue_x 100.0) _returnvalue_y _returnvalue_z) false false)
      (goto _label_13))))

(event `RockMovedRight`
  ;[0.2 0.2 0.2] Right
  (goto _label_12))

(fn `UserConstructionScript`)